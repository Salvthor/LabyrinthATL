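; BP_DoorSpawner is an actor that places two BP_Door actors at random spawn transforms when play begins.
; Each pass picks a transform from AvailableSpawns, spawns a door there, and removes that transform from the list so it is not picked again.
; Each door takes its ID from the incrementing DoorsID counter, then refreshes its text through UpdateDoorText.
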(event EventBeginPlay
  (bind _doorsid (Variables|Default|GetDoorsID))
  (for _index (range 0 1)
    (bind _output_get (Variables|Default|SetcurrentSpawn (.OutItem (Utilities|Array|Random (Variables|Default|GetAvailable%20Spawns)))))
    (bind _returnvalue (Game|SpawnActorfromClass "/Game/Environment/BP_Doors/BP_Door.BP_Door_C" _output_get "Undefined" "MultiplyWithRoot" 0 0))
    (Variables|/Game/Environment/BP_Doors/Overlappable.Overlappable_C|SetID _returnvalue _doorsid)
    (Math|Integer|IncrementInt _doorsid
      (:%20%20
        (Default|UpdateDoorText _returnvalue)
        (Utilities|Array|RemoveItem (Variables|Default|GetAvailable%20Spawns) (Variables|Default|GetcurrentSpawn))))))

(event Collision|EventActorBeginOverlap
  (params (OtherActor :type Actor%20Object%20Reference)))

(event EventTick
  (params (DeltaSeconds :type Float%20%28single-precision%29)))

(fn ConstructionScript)