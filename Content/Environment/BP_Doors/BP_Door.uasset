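; Labyrinth door Blueprint that swings shut once and reports the closure to the game mode.
; OverlapAction sets DoorClosed and plays DoorTimeline in reverse from the end to drive the door's yaw.
; When the timeline finishes, the Box stops generating overlap events and LabyrinthGM receives ClosedDoorNotify.
; UpdateDoorText labels the door with its one-based ID and fixes the text's world rotation.
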(event EventBeginPlay)

(event Collision|EventActorBeginOverlap
  (params (OtherActor :type Actor%20Object%20Reference)))

(event EventTick
  (params (DeltaSeconds :type Float%20%28single-precision%29)))

(event EventOverlapAction
  (if (not (Variables|Default|GetDoorClosed))
    (Variables|Default|SetDoorClosed true)
    (bind _doorrotationz (Timeline|DoorTimeline ReverseFromEnd)
      (:Update
        (Transformation|SetRelativeRotation (Variables|Default|GetDoor) (Math|Rotator|MakeRotator 0.0 0.0 _doorrotationz) false false))
      (:Finished
        (Variables|/Script/Engine.PrimitiveComponent|SetbGenerateOverlapEvents (Variables|Default|GetBox) false)
        (bind _aslabyrinth_gm (Utilities|Casting|CastToLabyrinthGM (Game|GetGameMode)))
        (Default|ClosedDoorNotify _aslabyrinth_gm)))))

(fn ConstructionScript)

(fn UpdateDoorText
  (bind _textrender (Variables|Default|GetTextRender))
  (Rendering|Components|TextRender|SetText _textrender (Utilities|Text|ToText(String) (Utilities|String|BuildString(Integer) "Door " "" (+ (Variables|Default|GetID) 1))))
  (Transformation|SetWorldRotation _textrender "90.000000,0.000000,180.000000" false false))